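; Mod main Blueprint that strips all non-player entities from the game.
; Every Tick it gathers all Character actors, filters out BPCharacter_Demo players and destroys the rest.
; It then removes spawn triggers in the Pipes and Level Run levels, plus cheat triggers in Level Run, using per-level flags to do so once.
; The mod button handler has no actions.
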(event `self.ReceiveTick`
  (params (DeltaSeconds :type "Float (single-precision)"))
  ;[1 1 1 1 16] Initial Operation
  ;[1 1 1 1 16] Gets all Entities And then remove
  (`self.Get And Set Entities`))

(fn `ModButtonWasPressed`
  (params (FunctionIndex :type Integer))
  (switch `int` FunctionIndex))

(fn `UserConstructionScript`
  (`parent.UserConstructionScript`))